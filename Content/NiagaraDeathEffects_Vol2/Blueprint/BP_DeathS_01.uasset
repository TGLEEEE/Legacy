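; Demo trigger actor that spawns a configurable death effect actor, named for burning and freezing on the map.
; Overlap of the box by the ThirdPersonCharacter enables input from player 0.
; Pressing E or V then waits a set delay and spawns the chosen class at the sphere component's transform.
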(event OnComponentBeginOverlap(Box)
  (params (OverlappedComponent :type Primitive%20Component%20Object%20Reference) (OtherActor :type Actor%20Object%20Reference) (OtherComp :type Primitive%20Component%20Object%20Reference) (OtherBodyIndex :type Integer) (bFromSweep :type Boolean) (SweepResult :type Hit%20Result%20Structure%20%28by%20ref%29))
  ;[1 1 1] Enable Input
  (Utilities|Casting|CastToThirdPersonCharacter OtherActor)
  (Input|EnableInput (Game|GetPlayerController 0)))

(event Input|KeyboardEvents|V
  (params (Key :type Key%20Structure :default "None"))
  (:Pressed
    (Utilities|FlowControl|Delay (Variables|Default|GetFirstDelay))
    ;[1 1 1] Spawn Actor For Burning And Freezing on Map
    (Game|SpawnActorfromClass (Variables|Default|GetClass) (Transformation|GetWorldTransform (Variables|Default|GetSphere)) "Undefined" 0 0)))

(event Input|KeyboardEvents|E
  (params (Key :type Key%20Structure :default "None"))
  (:Pressed
    (Utilities|FlowControl|Delay (Variables|Default|GetFirstDelay))
    ;[1 1 1] Spawn Actor For Burning And Freezing on Map
    (Game|SpawnActorfromClass (Variables|Default|GetClass) (Transformation|GetWorldTransform (Variables|Default|GetSphere)) "Undefined" 0 0)))

(fn ConstructionScript)