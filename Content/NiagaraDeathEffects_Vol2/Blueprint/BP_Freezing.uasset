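; BP_Freezing is a death effect that, on BeginPlay, freezes a skeletal mesh, shatters it and removes the actor.
; After a delay it pauses animation, disables collision, attaches ice Niagara and swaps to a material whose radius parameters a timeline animates.
; It then hides the mesh and breaks an added destructible component with radius damage.
; A second timeline drives a colored dissolve on the debris, with DestroyActor ending the effect.
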(event EventBeginPlay
  ;[1 1 1] Freezing Effect
  (|Freezing))

(fn ConstructionScript)

(fn DissoleMatParam
  (params (ParameterValue :type Float%20%28single-precision%29) (InputPin :type Mesh%20Component%20Object%20Reference))
  (Rendering|Material|SetScalarParameterValueonMaterials InputPin "Dissolve" ParameterValue)
  (Rendering|Material|SetVectorParameterValueonMaterials InputPin "color" (Math|Conversions|ToVector(LinearColor) (Variables|Default|GetColor))))