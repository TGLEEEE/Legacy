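; Burning death-effect Blueprint that sets a skeletal mesh alight on BeginPlay.
; After an initial delay, it attaches a Niagara system to the mesh and swaps every material slot to a burn material.
; A timeline animates the Dissolve and BodyColor parameters.
; A delay chained off that timeline's updates then deactivates the Niagara system and plays a second "Back To Normal" timeline on the same parameters.
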(event EventBeginPlay
  ;[1 1 1] Burning Body
  (|Burning))

(fn ConstructionScript)