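; Crypt double-door actor that swings open on the first overlap of its trigger box and starts the game.
; The overlap sets an opening flag, then after a short delay sets IsGameStart on the BP_LegacyGameMode cached at BeginPlay.
; While opening, Tick lerps both door leaves from their current rotation with an accumulating timer as alpha, stopping just short of full alpha.
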(event OnComponentBeginOverlap(Box)
  (params (OverlappedComponent :type Primitive%20Component%20Object%20Reference) (OtherActor :type Actor%20Object%20Reference) (OtherComp :type Primitive%20Component%20Object%20Reference) (OtherBodyIndex :type Integer) (bFromSweep :type Boolean) (SweepResult :type Hit%20Result%20Structure%20%28by%20ref%29))
  (Utilities|FlowControl|DoOnce false
    (:Completed
      (Variables|Default|SetIsOpening true)
      (Utilities|FlowControl|Delay 1.0)
      (Variables|/Script/Legacy.LegacyGameMode|SetbIsGameStart (Variables|Default|GetAs%20BP%20Legacy%20Game%20Mode) true))))

(event EventBeginPlay
  (bind _asbp_legacy_game_mode (Utilities|Casting|CastToBP_LegacyGameMode (Game|GetGameMode)))
  (Variables|Default|SetAs%20BP%20Legacy%20Game%20Mode _asbp_legacy_game_mode))

(event Collision|EventActorBeginOverlap
  (params (OtherActor :type Actor%20Object%20Reference)))

(event EventTick
  (params (DeltaSeconds :type Float%20%28single-precision%29))
  (bind _sm_doorway_large_door_left (Variables|Default|GetSM_DoorWay_Large_Door_Left))
  (bind _sm_doorway_large_door_right (Variables|Default|GetSM_DoorWay_Large_Door_Right))
  (if (Variables|Default|GetIsOpening)
    (Variables|Default|SetAlphaTimer (+ DeltaSeconds (Variables|Default|GetAlphaTimer)))
    (Transformation|SetRelativeRotation _sm_doorway_large_door_left (Math|Rotator|Lerp(Rotator) (Variables|/Script/Engine.SceneComponent|GetRelativeRotation _sm_doorway_large_door_left) "0.000000,-180.000000,0.000000" (Variables|Default|GetAlphaTimer)) false false)
    (Transformation|SetRelativeRotation _sm_doorway_large_door_right (Math|Rotator|Lerp(Rotator) (Variables|/Script/Engine.SceneComponent|GetRelativeRotation _sm_doorway_large_door_right) "0, 0, 0" (Variables|Default|GetAlphaTimer)) false false)
    (if (>= (Variables|Default|GetAlphaTimer) 0.9)
      (Variables|Default|SetIsOpening false))))

(fn ConstructionScript)